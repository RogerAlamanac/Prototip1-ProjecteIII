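; NPC patient Blueprint that carries a disease and exposes per-body-part symptoms for diagnosis and medication.
; InitialiseSyntoms rebuilds the symptom array from DeseaseName (Toothache, Migraines, Bleeding), randomising whether some symptoms are present.
; GetSymptoms returns only the first entry matching a body part, though one part gets two entries.
; ReceiveMedication looks up the required medicine in GI_GameInstance and only prints it; event graph and construction script are empty.
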(event EventBeginPlay)

(event Collision|EventActorBeginOverlap
  (params (OtherActor :type Actor%20Object%20Reference)))

(event EventTick
  (params (DeltaSeconds :type Float%20%28single-precision%29)))

(fn ConstructionScript)

(fn ReceiveMedication
  (bind _asgi_game_instance (Utilities|Casting|CastToGI_GameInstance (Game|GetGameInstance)))
  (bind _medicinerequired (Default|GetRequiredMedicine _asgi_game_instance (Variables|Default|GetDeseaseName)))
  (Development|PrintText (Utilities|Text|ToText(String) (Utilities|String|EnumtoString _medicinerequired))))

(fn InizialiseSyntoms
  (Utilities|Array|Clear (Variables|Default|GetBodyPartSyntoms))
  (switch Utilities|FlowControl|Switch|SwitchonE_DiseasesName (Variables|Default|GetDeseaseName)
    (:NewEnumerator0
      (Utilities|Array|Add (Variables|Default|GetBodyPartSyntoms) (Utilities|Struct|MakeST_SyntomsBodyPart "NewEnumerator0" true "Jaw Pain"))
      (Utilities|Array|Add (Variables|Default|GetBodyPartSyntoms) (Utilities|Struct|MakeST_SyntomsBodyPart "NewEnumerator1" (<= (Math|Random|RandomIntegerinRange 0 100) 30) "Muscular Tension"))
      (Utilities|Array|Add (Variables|Default|GetBodyPartSyntoms) (Utilities|Struct|MakeST_SyntomsBodyPart "NewEnumerator1" true "Low Feber"))
      (Utilities|Array|Add (Variables|Default|GetBodyPartSyntoms) (Utilities|Struct|MakeST_SyntomsBodyPart "NewEnumerator2" false "No Symptoms")))
    (:NewEnumerator1
      (Utilities|Array|Add (Variables|Default|GetBodyPartSyntoms) (Utilities|Struct|MakeST_SyntomsBodyPart "NewEnumerator0" true "Malaise "))
      (Utilities|Array|Add (Variables|Default|GetBodyPartSyntoms) (Utilities|Struct|MakeST_SyntomsBodyPart "NewEnumerator1" (<= (Math|Random|RandomIntegerinRange 0 100) 30) "Muscular Tension"))
      (Utilities|Array|Add (Variables|Default|GetBodyPartSyntoms) (Utilities|Struct|MakeST_SyntomsBodyPart "NewEnumerator1" (<= (Math|Random|RandomIntegerinRange 0 100) 30) "Low Feber"))
      (Utilities|Array|Add (Variables|Default|GetBodyPartSyntoms) (Utilities|Struct|MakeST_SyntomsBodyPart "NewEnumerator2" false "No Symptoms")))
    (:NewEnumerator2
      (Utilities|Array|Add (Variables|Default|GetBodyPartSyntoms) (Utilities|Struct|MakeST_SyntomsBodyPart "NewEnumerator0" (<= (Math|Random|RandomIntegerinRange 0 100) 30) "Face Scar"))
      (Utilities|Array|Add (Variables|Default|GetBodyPartSyntoms) (Utilities|Struct|MakeST_SyntomsBodyPart "NewEnumerator1" (<= (Math|Random|RandomIntegerinRange 0 100) 30) "Internal Contusions"))
      (Utilities|Array|Add (Variables|Default|GetBodyPartSyntoms) (Utilities|Struct|MakeST_SyntomsBodyPart "NewEnumerator1" (<= (Math|Random|RandomIntegerinRange 0 100) 30) "Low Feber"))
      (Utilities|Array|Add (Variables|Default|GetBodyPartSyntoms) (Utilities|Struct|MakeST_SyntomsBodyPart "NewEnumerator2" (<= (Math|Random|RandomIntegerinRange 0 100) 30) "Infected Cut")))))

(fn GetSymptoms
  (params (BodyPart :type E_BodyParts%20Enum :default "NewEnumerator0"))
  (for _array_element (Variables|Default|GetBodyPartSyntoms)
    (if (== (.BodyPart (Utilities|Struct|BreakST_SyntomsBodyPart _array_element)) (Math|Conversions|ToInteger(Byte) BodyPart))
      (bind _output_get (LocalVariables|SetTemp_HasSymptom (.hasSyntom (Utilities|Struct|BreakST_SyntomsBodyPart _array_element))))
      (bind _output_get_2 (LocalVariables|SetTemp_Description (.Description (Utilities|Struct|BreakST_SyntomsBodyPart _array_element))))
      (return _output_get _output_get_2))))